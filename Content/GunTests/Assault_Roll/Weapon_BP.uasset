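; Assault rifle weapon Blueprint with automatic primary fire and a shotgun secondary, each with its own ammo.
; Both fire events animate the player's arms, spawn one FirstPersonProjectile at the barrel socket, then re-call themselves after a delay while the button is held.
; Primary adds a random muzzle flash; secondary animates the shotgun mesh and gates on CanFire.
; An alternative timer-driven fire path is marked broken, and PrimaryFire partly duplicates Fire.
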(event Custom|Fire
  (bind _primary_muzzle (Variables|Default|GetPrimary_Muzzle))
  ;[1 1 1] Primary Fire
  (if (> (Variables|Default|GetAmmo) 0)
    (bind _asfirst_person_character (Utilities|Casting|CastToFirstPersonCharacter (Game|Player|GetPlayerPawn 0)))
    (Components|Animation|PlayAnimation (Variables|/Game/FirstPersonBP/Blueprints/FirstPersonCharacter.FirstPersonCharacter_C|GetMesh2P _asfirst_person_character) "/Game/FPArms/FPArms_AR_FullAuto_Anim.FPArms_AR_FullAuto_Anim" false)
    (Game|SpawnActorfromClass "/Game/GunTests/Assault_Roll/FirstPersonProjectile.FirstPersonProjectile_C" (Transformation|GetSocketTransform (Variables|Default|GetAR_Body) "CylinderSocket" "RTS_World") "Undefined" 0 0)
    (Variables|Default|SetAmmo (- (Variables|Default|GetAmmo) 1))
    (bind _asfirst_person_character_2 (Utilities|Casting|CastToFirstPersonCharacter (Game|Player|GetPlayerPawn 0)))
    (Effects|SpawnEmitteratLocation (Utilities|Array|Get(acopy) _primary_muzzle (Math|Random|RandomInteger (Utilities|Array|Length _primary_muzzle))) (Transformation|GetSocketLocation (Variables|Weapon_BP_C|GetAR_Body (Variables|/Game/FirstPersonBP/Blueprints/FirstPersonCharacter.FirstPersonCharacter_C|GetCurrent_Weapon _asfirst_person_character_2)) "CylinderSocket") (Transformation|GetWorldRotation (Variables|/Game/FirstPersonBP/Blueprints/FirstPersonCharacter.FirstPersonCharacter_C|GetFirstPersonCamera _asfirst_person_character_2)))
    (Utilities|FlowControl|Delay (Variables|Default|GetFireRate))
    (if (> (Variables|Default|GetAmmo) 0)
      (bind _asfirst_person_character_3 (Utilities|Casting|CastToFirstPersonCharacter (Game|Player|GetPlayerPawn 0)))
      (if (Variables|/Game/FirstPersonBP/Blueprints/FirstPersonCharacter.FirstPersonCharacter_C|GetFireButtonHeld _asfirst_person_character_3)
        (CallFunction|Fire)))))

(event Custom|Idle%20Animation
  ;[1 1 1] Primary Idle Animation
  (bind _asfirst_person_character (Utilities|Casting|CastToFirstPersonCharacter (Game|Player|GetPlayerPawn 0)))
  (Components|Animation|PlayAnimation (Variables|/Game/FirstPersonBP/Blueprints/FirstPersonCharacter.FirstPersonCharacter_C|GetMesh2P _asfirst_person_character) "/Game/FPArms/FPArms_AR_Idle_01.FPArms_AR_Idle_01" true))

(event Custom|Secondary%20Idle
  ;[1 1 1] Secondary Idle Animation
  (Utilities|FlowControl|Delay 1.0)
  (bind _asfirst_person_character (Utilities|Casting|CastToFirstPersonCharacter (Game|Player|GetPlayerPawn 0)))
  (Components|Animation|PlayAnimation (Variables|/Game/FirstPersonBP/Blueprints/FirstPersonCharacter.FirstPersonCharacter_C|GetMesh2P _asfirst_person_character) "/Game/FPArms/FPArms_AR_Idle_01.FPArms_AR_Idle_01" false))

(event Custom|PlayerShooting
  ;[1 1 1] Shit that don't fukin work
  (bind _returnvalue (Utilities|Time|SetTimerbyFunctionName 0 "Shooting" 0.06 true)))

(event Custom|PlayerNotShooting
  ;[1 1 1] Shit that don't fukin work
  (Utilities|Time|ClearandInvalidateTimerbyHandle (stale Custom|PlayerShooting _returnvalue)))

(event Custom|Secondary%20Fire
  ;[1 1 1] Secondary Fire
  (if (Variables|Default|GetCanFire)
    (if (> (Variables|Default|GetSecondary%20Ammo) 0)
      (bind _asfirst_person_character (Utilities|Casting|CastToFirstPersonCharacter (Game|Player|GetPlayerPawn 0)))
      (Components|Animation|PlayAnimation (Variables|/Game/FirstPersonBP/Blueprints/FirstPersonCharacter.FirstPersonCharacter_C|GetMesh2P _asfirst_person_character) "/Game/FPArms/FPArms_AR_Shotgun.FPArms_AR_Shotgun" false)
      (Components|Animation|PlayAnimation (Variables|Default|GetAR_Shotty) "/Game/GunTests/Assault_Roll/AR_Shotgun_Anim.AR_Shotgun_Anim" false)
      (Game|SpawnActorfromClass "/Game/GunTests/Assault_Roll/FirstPersonProjectile.FirstPersonProjectile_C" (Transformation|GetSocketTransform (Variables|Default|GetAR_Body) "CylinderSocket" "RTS_World") "Undefined" 0 0)
      (Variables|Default|SetSecondary%20Ammo (- (Variables|Default|GetSecondary%20Ammo) 1))
      (Variables|Default|SetCanFire false)
      (Utilities|FlowControl|Delay 1.0)
      (Variables|Default|SetCanFire true)
      (bind _asfirst_person_character_2 (Utilities|Casting|CastToFirstPersonCharacter (Game|Player|GetPlayerPawn 0)))
      (if (Variables|/Game/FirstPersonBP/Blueprints/FirstPersonCharacter.FirstPersonCharacter_C|GetSecondaryFireHeld _asfirst_person_character_2)
        (CallFunction|SecondaryFire)))))

(event Collision|EventActorBeginOverlap
  (params (OtherActor :type Actor%20Object%20Reference)))

(fn ConstructionScript)

(fn Shooting
  (CallFunction|Fire))

(fn PrimaryFire
  (if (> (Variables|Default|GetAmmo) 0)
    (bind _asfirst_person_character (Utilities|Casting|CastToFirstPersonCharacter (Game|Player|GetPlayerPawn 0)))
    (Components|Animation|PlayAnimation (Variables|/Game/FirstPersonBP/Blueprints/FirstPersonCharacter.FirstPersonCharacter_C|GetMesh2P _asfirst_person_character) "/Game/FPArms/FPArms_AR_FullAuto_Anim.FPArms_AR_FullAuto_Anim" false)
    (Game|SpawnActorfromClass "/Game/GunTests/Assault_Roll/FirstPersonProjectile.FirstPersonProjectile_C" (Transformation|GetSocketTransform (Variables|Default|GetAR_Body) "CylinderSocket" "RTS_World") "Undefined" 0 0)
    (Variables|Default|SetAmmo (- (Variables|Default|GetAmmo) 1))
    (if (> (Variables|Default|GetAmmo) 0)
      (bind _asfirst_person_character_2 (Utilities|Casting|CastToFirstPersonCharacter (Game|Player|GetPlayerPawn 0)))
      (if (Variables|/Game/FirstPersonBP/Blueprints/FirstPersonCharacter.FirstPersonCharacter_C|GetFireButtonHeld _asfirst_person_character_2)
        (CallFunction|Fire)))))

(fn PrimaryIdle
  (bind _asfirst_person_character (Utilities|Casting|CastToFirstPersonCharacter (Game|Player|GetPlayerPawn 0)))
  (Components|Animation|PlayAnimation (Variables|/Game/FirstPersonBP/Blueprints/FirstPersonCharacter.FirstPersonCharacter_C|GetMesh2P _asfirst_person_character) "/Game/FPArms/FPArms_AR_Idle_01.FPArms_AR_Idle_01" false))