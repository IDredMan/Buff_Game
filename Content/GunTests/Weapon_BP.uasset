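; Weapon Blueprint for an automatic rifle that fires projectiles and drives the first-person character's arm animations.
; PlayerShooting starts a fast looping timer on the Shooting function, which calls Fire until PlayerNotShooting clears the timer.
; Fire plays the full-auto arm animation on player 0's Mesh2P and spawns FirstPersonProjectile at the ARBody cylinder socket.
; IdleAnimation loops the arms' idle, while the weapon-body animation nodes are left unconnected.
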(event Custom|Fire
  (bind _asfirst_person_character (Utilities|Casting|CastToFirstPersonCharacter (Game|Player|GetPlayerPawn 0)))
  (Components|Animation|PlayAnimation (Variables|/Game/FirstPersonBP/Blueprints/FirstPersonCharacter.FirstPersonCharacter_C|GetMesh2P _asfirst_person_character) "/Game/FPArms_AR_FullAuto_Anim.FPArms_AR_FullAuto_Anim" false)
  (Game|SpawnActorfromClass "/Game/FirstPersonBP/Blueprints/FirstPersonProjectile.FirstPersonProjectile_C" (Transformation|GetSocketTransform (Variables|Default|GetAR_Body) "CylinderSocket" "RTS_World") "Undefined" 0 0))

(event Custom|Idle%20Animation
  (bind _asfirst_person_character (Utilities|Casting|CastToFirstPersonCharacter (Game|Player|GetPlayerPawn 0)))
  (Components|Animation|PlayAnimation (Variables|/Game/FirstPersonBP/Blueprints/FirstPersonCharacter.FirstPersonCharacter_C|GetMesh2P _asfirst_person_character) "/Game/Characters/FPArms_AR_Idle_01.FPArms_AR_Idle_01" true))

(event Custom|PlayerShooting
  (bind _returnvalue (Utilities|Time|SetTimerbyFunctionName 0 "Shooting" 0.06 true)))

(event Custom|PlayerNotShooting
  (Utilities|Time|ClearandInvalidateTimerbyHandle (stale Custom|PlayerShooting _returnvalue)))

(event EventBeginPlay)

(event Collision|EventActorBeginOverlap
  (params (OtherActor :type Actor%20Object%20Reference)))

(event EventTick
  (params (DeltaSeconds :type Float%20%28single-precision%29)))

(fn ConstructionScript)

(fn Shooting
  (CallFunction|Fire))